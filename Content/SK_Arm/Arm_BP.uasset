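; Arm Blueprint that lets the player pose a skeletal arm from the keyboard through a Control Rig mapped to its mesh in the construction script.
; Held Q/E, A/D and W/S keys run looping timers that step roll, pitch and yaw on three separate bone controls.
; Z toggles a timer that moves the Cube to the end control's rig-space location, simulating a grab without physics or proximity checks.
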(event Custom|RotatorE
  (bind _controlrig (Variables|Default|GetControlRig))
  (bind _returnvalue (Class|ControlRigComponent|GetControlRotator _controlrig "Bone_001Ctrl" "LocalSpace"))
  (Class|ControlRigComponent|SetControlRotator (Variables|Default|GetControlRig) "Bone_001Ctrl" (Math|Rotator|MakeRotator (+ -5.0 (.roll _returnvalue)) (.pitch _returnvalue) (.yaw _returnvalue)) "LocalSpace"))

(event Custom|RotatorW
  (bind _controlrig (Variables|Default|GetControlRig))
  (bind _returnvalue (Class|ControlRigComponent|GetControlRotator _controlrig "Bone_000Ctrl" "LocalSpace"))
  (Class|ControlRigComponent|SetControlRotator (Variables|Default|GetControlRig) "Bone_000Ctrl" (Math|Rotator|MakeRotator (.roll _returnvalue) (.pitch _returnvalue) (+ -5.0 (.yaw _returnvalue))) "LocalSpace"))

(event Custom|RotatorD
  (bind _controlrig (Variables|Default|GetControlRig))
  (bind _returnvalue (Class|ControlRigComponent|GetControlRotator _controlrig "Bone_002Ctrl" "LocalSpace"))
  (bind _returnvalue_2 (+ -5.0 (.pitch _returnvalue)))
  (Class|ControlRigComponent|SetControlRotator (Variables|Default|GetControlRig) "Bone_002Ctrl" (Math|Rotator|MakeRotator (.roll _returnvalue) _returnvalue_2 (.yaw _returnvalue)) "LocalSpace")
  (Development|PrintString (Utilities|String|ToString(Float) _returnvalue_2)))

(event Custom|RotatorA
  (bind _controlrig (Variables|Default|GetControlRig))
  (bind _returnvalue (Class|ControlRigComponent|GetControlRotator _controlrig "Bone_002Ctrl" "LocalSpace"))
  (Class|ControlRigComponent|SetControlRotator (Variables|Default|GetControlRig) "Bone_002Ctrl" (Math|Rotator|MakeRotator (.roll _returnvalue) (+ 5.0 (.pitch _returnvalue)) (.yaw _returnvalue)) "LocalSpace"))

(event Custom|RotatorQ
  (bind _controlrig (Variables|Default|GetControlRig))
  (bind _returnvalue (Class|ControlRigComponent|GetControlRotator _controlrig "Bone_001Ctrl" "LocalSpace"))
  (Class|ControlRigComponent|SetControlRotator (Variables|Default|GetControlRig) "Bone_001Ctrl" (Math|Rotator|MakeRotator (+ 5.0 (.roll _returnvalue)) (.pitch _returnvalue) (.yaw _returnvalue)) "LocalSpace"))

(event Custom|RotatorS
  (bind _controlrig (Variables|Default|GetControlRig))
  (bind _returnvalue (Class|ControlRigComponent|GetControlRotator _controlrig "Bone_000Ctrl" "LocalSpace"))
  (Class|ControlRigComponent|SetControlRotator (Variables|Default|GetControlRig) "Bone_000Ctrl" (Math|Rotator|MakeRotator (.roll _returnvalue) (.pitch _returnvalue) (+ 5.0 (.yaw _returnvalue))) "LocalSpace"))

(event Custom|grabbing
  (Transformation|SetRelativeLocation (Variables|Default|GetCube) (.location (Class|ControlRigComponent|GetControlTransform (Variables|Default|GetControlRig) "Bone_007_endCtrl" "RigSpace")) false false))

(event Input|KeyboardEvents|W
  (params (Key :type Key%20Structure :default "None"))
  (:Pressed
    (Utilities|Time|SetTimerbyEvent (delegate Custom|RotatorW) 0.1 true))
  (:Released
    (Utilities|Time|ClearTimerbyFunctionName 0 "RotatorW")))

(event Input|KeyboardEvents|D
  (params (Key :type Key%20Structure :default "None"))
  (:Pressed
    (Utilities|Time|SetTimerbyEvent (delegate Custom|RotatorD) 0.1 true))
  (:Released
    (Utilities|Time|ClearTimerbyFunctionName 0 "RotatorD")))

(event Input|KeyboardEvents|A
  (params (Key :type Key%20Structure :default "None"))
  (:Pressed
    (Utilities|Time|SetTimerbyEvent (delegate Custom|RotatorA) 0.1 true))
  (:Released
    (Utilities|Time|ClearTimerbyFunctionName 0 "RotatorA")))

(event Input|KeyboardEvents|Q
  (params (Key :type Key%20Structure :default "None"))
  (:Pressed
    (Utilities|Time|SetTimerbyEvent (delegate Custom|RotatorQ) 0.1 true))
  (:Released
    (Utilities|Time|ClearTimerbyFunctionName 0 "RotatorQ")))

(event Input|KeyboardEvents|E
  (params (Key :type Key%20Structure :default "None"))
  (:Pressed
    (Utilities|Time|SetTimerbyEvent (delegate Custom|RotatorE) 0.1 true))
  (:Released
    (Utilities|Time|ClearTimerbyFunctionName 0 "RotatorE")))

(event Input|KeyboardEvents|Z
  (params (Key :type Key%20Structure :default "None"))
  (:Pressed
    (if (Variables|Default|GetIsGrabbing)
      (Variables|Default|SetIsGrabbing false)
      (Utilities|Time|ClearTimerbyFunctionName 0 "grabbing")
      (else
        (Variables|Default|SetIsGrabbing true)
        (Utilities|Time|SetTimerbyEvent (delegate Custom|grabbing) 0.1 true)))))

(event Input|KeyboardEvents|S
  (params (Key :type Key%20Structure :default "None"))
  (:Pressed
    (Utilities|Time|SetTimerbyEvent (delegate Custom|RotatorS) 0.1 true))
  (:Released
    (Utilities|Time|ClearTimerbyFunctionName 0 "RotatorS")))

(fn ConstructionScript
  (Class|ControlRigComponent|AddMappedCompleteSkeletalMesh (Variables|Default|GetControlRig) (Variables|Default|GetSkeletalMesh)))